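; BP_FallingObstacle is an obstacle actor that fades out and destroys itself once the player touches it.
; When BP_Player overlaps its Box, a looping 0.01-second timer starts calling DecreaseOpacity.
; Each tick lowers the Opacity variable by OpacityToDecrease and pushes it to the Cube's material scalar parameter, clearing the timer and destroying the actor at zero.
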(event OnComponentBeginOverlap(Box)
  (params (OverlappedComponent :type Primitive%20Component%20Object%20Reference) (OtherActor :type Actor%20Object%20Reference) (OtherComp :type Primitive%20Component%20Object%20Reference) (OtherBodyIndex :type Integer) (bFromSweep :type Boolean) (SweepResult :type Hit%20Result%20Structure%20%28by%20ref%29))
  (Utilities|Casting|CastToBP_Player OtherActor)
  (Utilities|Time|SetTimerbyFunctionName 0 "DecreaseOpacity" 0.01 true))

(fn ConstructionScript)

(fn DecreaseOpacity
  (Variables|Default|SetOpacity (- (Variables|Default|GetOpacity) (Variables|Default|GetOpacityToDecrease)))
  (Rendering|Material|SetScalarParameterValueonMaterials (Variables|Default|GetCube) "Opacity" (Variables|Default|GetOpacity))
  (if (<= (Variables|Default|GetOpacity) 0.0)
    (Utilities|Time|ClearTimerbyFunctionName 0 "DecreaseOpacity")
    (Actor|DestroyActor)))