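; BP_CheckPoint is a checkpoint actor that updates the player's respawn point and can end the game.
; When BP_Player enters its box trigger, it sets the player's RespawnTransform to the Arrow component's location and rotation at unit scale.
; If flagged as the last checkpoint, it also marks the player as having won and adds the WB_EndScreen widget to the viewport.
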(event OnComponentBeginOverlap(Box)
  (params (OverlappedComponent :type Primitive%20Component%20Object%20Reference) (OtherActor :type Actor%20Object%20Reference) (OtherComp :type Primitive%20Component%20Object%20Reference) (OtherBodyIndex :type Integer) (bFromSweep :type Boolean) (SweepResult :type Hit%20Result%20Structure%20%28by%20ref%29))
  (bind _arrow (Variables|Default|GetArrow))
  (bind _returnvalue (Transformation|GetWorldTransform _arrow))
  (bind (_location _rotation) (Math|Transform|BreakTransform _returnvalue))
  ;[1 1 1] Set respawn du personnage sur la flèche
  (bind _asbp_player (Utilities|Casting|CastToBP_Player OtherActor))
  (Variables|/Game/Blueprints/Characters/BP_Player.BP_Player_C|SetRespawnTransform _asbp_player (Math|Transform|MakeTransform _location _rotation))
  (if (Variables|Default|GetIsLastCheckPoint)
    (Default|SetWin _asbp_player true)
    (bind _returnvalue_2 (UserInterface|CreateWidget "/Game/Blueprints/UI/WB_EndScreen.WB_EndScreen_C"))
    (UserInterface|Viewport|AddtoViewport _returnvalue_2 0)))

(fn ConstructionScript)